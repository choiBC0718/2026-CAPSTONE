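; BP_HellGate is a hell gate actor that F_ToggleHellGate switches on and off with timed visual and audio transitions, ignoring calls mid-transition.
; Looping timers step a shared TransitionFloat to drive dynamic material parameters, light intensity and volume.
; Activation has two phases: gate emission rises as orb effects start in turn, then fire and screams start while the portal fades in.
; Deactivation stops fire and orbs, then fades everything out together.
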(event EventBeginPlay
  (bind _returnvalue (Rendering|Material|CreateDynamicMaterialInstance (Variables|Default|GetHellGate_HellGate) 0 0 "None" :!class /Script/Engine.PrimitiveComponent))
  (bind _output_get (Variables|Default|SetMID_HellGate _returnvalue))
  (bind _returnvalue_2 (Rendering|Material|CreateDynamicMaterialInstance (Variables|Default|GetHellGate_HellGate_Portal) 0 0 "None" :!class /Script/Engine.PrimitiveComponent))
  (bind _output_get_2 (Variables|Default|SetMID_Portal _returnvalue_2))
  (Rendering|Material|SetScalarParameterValue _output_get "Emission_Amount" 0.0 :!class /Script/Engine.MaterialInstanceDynamic)
  (Rendering|Material|SetScalarParameterValue _output_get_2 "Alpha_Cutof" 1.0 :!class /Script/Engine.MaterialInstanceDynamic)
  (Rendering|Components|Light|SetIntensity (Variables|Default|GetLight_Gate) 0.0)
  (Components|Activation|SetActive (Variables|Default|GetHellGate_HellGate_Portal) false false))

(fn ConstructionScript)

(fn FToggleHellGate
  (if (not (Variables|Default|GetinTransition))
    (Variables|Default|SetinTransition true)
    (if (Variables|Default|GetisActivated)
      (Components|Activation|Deactivate (Variables|Default|GetPS_Gate_Fire))
      (Components|Activation|Deactivate (Variables|Default|GetPS_OrbL))
      (Components|Activation|Deactivate (Variables|Default|GetPS_OrbR))
      (Audio|Components|Audio|Stop (Variables|Default|GetSC_Gate_Fire))
      (bind _returnvalue (Utilities|Time|SetTimerbyFunctionName 0 "F_DeActivate" 0.03 true))
      (Variables|Default|Settransition_TH _returnvalue)
      (else
        (bind _returnvalue_2 (Utilities|Time|SetTimerbyFunctionName 0 "F_PreActivate" 0.03 true))
        (Variables|Default|Settransition_TH _returnvalue_2)))))

(fn FActivate
  (if (< (Variables|Default|GettransitionFloat) 1.0)
    ;[1 1 1] Timer
    (Variables|Default|SettransitionFloat (+ (Variables|Default|GettransitionFloat) 0.006))
    (Rendering|Material|SetScalarParameterValue (Variables|Default|GetMID_Portal) "Alpha_Cutof" (- 1.0 (Variables|Default|GettransitionFloat)) :!class /Script/Engine.MaterialInstanceDynamic)
    (Audio|Components|Audio|SetVolumeMultiplier (Variables|Default|GetSC_Smackeling) (* (Variables|Default|GettransitionFloat) 0.1) :!class /Script/Engine.AudioComponent)
    (Rendering|Components|Light|SetIntensity (Variables|Default|GetLight_Gate) (* (Variables|Default|GettransitionFloat) 5e+03))
    (else
      (Utilities|Time|ClearandInvalidateTimerbyHandle (Variables|Default|Gettransition_TH))
      (Variables|Default|SetinTransition false)
      (Variables|Default|SetisActivated true))))

(fn FDeActivate
  (if (> (Variables|Default|GettransitionFloat) 0.0)
    ;[1 1 1] Timer
    (Variables|Default|SettransitionFloat (- (Variables|Default|GettransitionFloat) 0.008))
    (Rendering|Material|SetScalarParameterValue (Variables|Default|GetMID_Portal) "Alpha_Cutof" (- 1.0 (Variables|Default|GettransitionFloat)) :!class /Script/Engine.MaterialInstanceDynamic)
    (Audio|Components|Audio|SetVolumeMultiplier (Variables|Default|GetSC_Smackeling) (* (Variables|Default|GettransitionFloat) 0.1) :!class /Script/Engine.AudioComponent)
    (Rendering|Components|Light|SetIntensity (Variables|Default|GetLight_Gate) (* (Variables|Default|GettransitionFloat) 5e+03))
    (Audio|Components|Audio|SetVolumeMultiplier (Variables|Default|GetSC_Gate_Fire) (* (Variables|Default|GettransitionFloat) 0.5) :!class /Script/Engine.AudioComponent)
    ;[1 1 1] Emission
    (Rendering|Material|SetScalarParameterValue (Variables|Default|GetMID_HellGate) "Emission_Amount" (Variables|Default|GettransitionFloat) :!class /Script/Engine.MaterialInstanceDynamic)
    (else
      (Utilities|Time|ClearandInvalidateTimerbyHandle (Variables|Default|Gettransition_TH))
      (Components|Activation|SetActive (Variables|Default|GetHellGate_HellGate_Portal) false false)
      (Variables|Default|SetinTransition false)
      (Variables|Default|SetisActivated false))))

(fn FPreActivate
  (bind _sc_gate_fire (Variables|Default|GetSC_Gate_Fire))
  (bind _ps_orbl (Variables|Default|GetPS_OrbL))
  (bind _ps_orbr (Variables|Default|GetPS_OrbR))
  (if (< (Variables|Default|GettransitionFloat) 1.0)
    ;[1 1 1] Timer
    (Variables|Default|SettransitionFloat (+ (Variables|Default|GettransitionFloat) 0.015))
    ;[1 1 1] Emission
    (Rendering|Material|SetScalarParameterValue (Variables|Default|GetMID_HellGate) "Emission_Amount" (Variables|Default|GettransitionFloat) :!class /Script/Engine.MaterialInstanceDynamic)
    ;[1 1 1] Activate OrbL
    (if (and (>= (Variables|Default|GettransitionFloat) 0.3) (not (Components|Activation|IsActive _ps_orbl)))
      (Components|Activation|Activate _ps_orbl false)
      (Audio|Components|Audio|Play (Variables|Default|GetSC_OrbL) 0.0)
      (else
        ;[1 1 1] Activate OrbR
        (if (and (>= (Variables|Default|GettransitionFloat) 0.6) (not (Components|Activation|IsActive _ps_orbr)))
          (Components|Activation|Activate _ps_orbr false)
          (Audio|Components|Audio|Play (Variables|Default|GetSC_OrbR) 0.0))))
    (else
      (Variables|Default|SettransitionFloat 0.0)
      (Components|Activation|Activate (Variables|Default|GetPS_Gate_Fire) false)
      (Audio|Components|Audio|Play (Variables|Default|GetSC_Screaming) 0.0)
      (Audio|Components|Audio|Play _sc_gate_fire 0.0)
      (Audio|Components|Audio|SetVolumeMultiplier _sc_gate_fire 0.5 :!class /Script/Engine.AudioComponent)
      (Audio|Components|Audio|Play (Variables|Default|GetSC_Smackeling) 0.0)
      (Components|Activation|SetActive (Variables|Default|GetHellGate_HellGate_Portal) true false)
      (Utilities|Time|ClearandInvalidateTimerbyHandle (Variables|Default|Gettransition_TH))
      (bind _returnvalue (Utilities|Time|SetTimerbyFunctionName 0 "F_Activate" 0.03 true))
      (Variables|Default|Settransition_TH _returnvalue))))