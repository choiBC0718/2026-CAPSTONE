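; Blood pool prop for a demonic altar set, switched on and off through F_ToggleBloodPool with torch fire, smoke, lights and sound.
; Toggling activates or deactivates the particles and starts a looping FadeEffects timer that ramps material emission and audio volume, dimming lights on fade-out.
; Once fully on, FlickerLights reschedules itself at random short intervals to vary both fire lights' intensity until the pool is toggled off.
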(event EventBeginPlay
  (bind _fire_light_left (Variables|Default|GetFire_Light_Left))
  (bind _returnvalue (Rendering|Material|CreateDynamicMaterialInstance (Variables|Default|GetSM_BloodPool) 0 0 "None" :!class /Script/Engine.PrimitiveComponent))
  (Variables|Default|SetMID_BloodPool _returnvalue)
  (Rendering|Material|SetScalarParameterValue (Variables|Default|GetMID_BloodPool) "Emission_Amount" 0.0 :!class /Script/Engine.MaterialInstanceDynamic)
  (Variables|Default|SetlightIntensityMax (Variables|/Script/Engine.LightComponentBase|GetIntensity _fire_light_left))
  (Rendering|Components|Light|SetIntensity _fire_light_left 0.0))

(fn ConstructionScript)

(fn FToggleBloodPool
  (Variables|Default|SetactivatePool (not (Variables|Default|GetactivatePool)))
  (if (Variables|Default|GetinTransition)
    _
    (else
      (Variables|Default|SetinTransition true)
      (bind _returnvalue (Utilities|Time|SetTimerbyFunctionName 0 "FadeEffects" 0.02 true))
      (Variables|Default|SetfadeEffectTH _returnvalue)))
  (if (Variables|Default|GetactivatePool)
    (Rendering|Components|Light|SetIntensity (Variables|Default|GetFire_Light_Left) (Variables|Default|GetlightIntensityMax))
    (Components|Activation|Activate (Variables|Default|GetPS_Fire_L1) true)
    (Audio|Components|Audio|Play (Variables|Default|GetSQ_TorchStart) 0.0)
    (else
      (Components|Activation|Deactivate (Variables|Default|GetPS_Fire_L)))))

(fn FadeEffects
  (if (Variables|Default|GetactivatePool)
    (Variables|Default|SettransitionFloat (Math|Float|Clamp(Float) (+ (Variables|Default|GettransitionFloat) 0.01)))
    (else
      (Variables|Default|SettransitionFloat (Math|Float|Clamp(Float) (- (Variables|Default|GettransitionFloat) 0.015)))
      (Rendering|Components|Light|SetIntensity (Variables|Default|GetFire_Light_Left) (* (Variables|Default|GetlightIntensityMax) (Variables|Default|GettransitionFloat)))))
  (Rendering|Material|SetScalarParameterValue (Variables|Default|GetMID_BloodPool) "Emission_Amount" (Variables|Default|GettransitionFloat) :!class /Script/Engine.MaterialInstanceDynamic)
  (Audio|Components|Audio|SetVolumeMultiplier (Variables|Default|GetSQ_TorchLoop) (* (Variables|Default|GettransitionFloat) 0.6) :!class /Script/Engine.AudioComponent)
  (Audio|Components|Audio|SetVolumeMultiplier (Variables|Default|GetSQ_Bubbles) (* (Variables|Default|GettransitionFloat) 0.4) :!class /Script/Engine.AudioComponent)
  (if (== (Variables|Default|GettransitionFloat) 0.0)
    (Audio|Components|Audio|Stop (Variables|Default|GetSQ_Bubbles))
    (Utilities|Time|ClearandInvalidateTimerbyHandle (Variables|Default|GetfadeEffectTH) :!label _label)
    (Variables|Default|SetinTransition false)
    (elif (== (Variables|Default|GettransitionFloat) 1.0)
      (Utilities|Time|SetTimerbyFunctionName 0 "FlickerLights" 1.0) ; Start Light Flicker Effect.
      (goto _label))))

(fn FlickerLights
  (bind _lightintensitymax (Variables|Default|GetlightIntensityMax))
  (Rendering|Components|Light|SetIntensity (Variables|Default|GetFire_Light_Right) (Math|Random|RandomFloatinRange (* _lightintensitymax 0.85) _lightintensitymax))
  (if (and (not (Variables|Default|GetinTransition)) (Variables|Default|GetactivatePool))
    (Utilities|Time|SetTimerbyFunctionName 0 "FlickerLights" (Math|Random|RandomFloatinRange 0.1 0.3))))