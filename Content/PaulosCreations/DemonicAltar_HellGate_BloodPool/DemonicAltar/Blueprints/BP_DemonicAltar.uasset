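; Demonic altar actor that toggles a hellish portal on and off with runes, particles, chanting and explosion audio, and lights.
; F_ToggleDemonicAltar starts looping timers that fade emission and portal light, spinning the rune circle before the portal bursts open, or fading it and its audio out.
; While active with LightningOn, a one-second timer triggers randomly delayed lightning strikes with a short light flicker.
; InTransition blocks re-toggling mid-transition.
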(event EventBeginPlay
  (bind _returnvalue (Rendering|Material|CreateDynamicMaterialInstance (Variables|Default|GetSM_DemonicAltar) 0 0 "None" :!class /Script/Engine.PrimitiveComponent))
  (Variables|Default|SetMID_DemonicAltar _returnvalue)
  (Rendering|Components|Light|SetIntensity (Variables|Default|GetLightning_Light) 0.0)
  (Rendering|Components|Light|SetIntensity (Variables|Default|GetPortal_Light) 0.0))

(fn ConstructionScript)

(fn FToggleDemonicAltar
  (if (not (Variables|Default|GetinTransition))
    (Variables|Default|SetinTransition true)
    (if (Variables|Default|GetisActivated)
      (if (Variables|Default|GetlightningOn)
        ;[1 1 1] Is lightning running ?
        (if (Utilities|Time|IsTimerActivebyHandle (Variables|Default|GetTH_runningTimer))
          (Utilities|Time|ClearandInvalidateTimerbyHandle (Variables|Default|GetTH_runningTimer))))
      (Components|Activation|Deactivate (Variables|Default|GetPS_Portal))
      (Variables|Default|SettransitionTimer 1.0)
      (bind _returnvalue (Utilities|Time|SetTimerbyFunctionName 0 "F_DeactivateAltar" 0.03 true))
      (Variables|Default|SetTH_runningTimer _returnvalue)
      (else
        (Components|Activation|Activate (Variables|Default|GetPS_RunesCircle) false)
        (Audio|Components|Audio|Play (Variables|Default|GetSC_Chanting) 0.0)
        (Variables|Default|SettransitionTimer 0.0)
        (bind _returnvalue_2 (Utilities|Time|SetTimerbyFunctionName 0 "F_Activate" 0.03 true))
        (Variables|Default|SetTH_runningTimer _returnvalue_2)))))

(fn FActivate
  (if (< (Variables|Default|GettransitionTimer) 1.0)
    (Variables|Default|SettransitionTimer (+ (Variables|Default|GettransitionTimer) 0.005))
    ;[1 1 1] Fade in Emission
    (Rendering|Material|SetScalarParameterValue (Variables|Default|GetMID_DemonicAltar) "Emission_Amount" (Variables|Default|GettransitionTimer) :!class /Script/Engine.MaterialInstanceDynamic)
    ;[1 1 1] Rotate rune circle
    (Transformation|AddLocalRotation (Variables|Default|GetPS_RunesCircle) (Math|Rotator|MakeRotator 0.0 0.0 (* (Variables|Default|GettransitionTimer) 1e+01)) false false)
    ;[1 1 1] Fade in portal light
    (Rendering|Components|Light|SetIntensity (Variables|Default|GetPortal_Light) (* (Variables|Default|GettransitionTimer) 1.5e+04))
    (else
      (Utilities|Time|ClearandInvalidateTimerbyHandle (Variables|Default|GetTH_runningTimer))
      (Components|Activation|Activate (Variables|Default|GetPS_RunesExplosion) false)
      (Audio|Components|Audio|Play (Variables|Default|GetSC_Explosion_Portal) 0.0)
      (Audio|Components|Audio|Stop (Variables|Default|GetSC_Chanting))
      (Components|Activation|Deactivate (Variables|Default|GetPS_RunesCircle))
      (Components|Activation|Activate (Variables|Default|GetPS_Portal) false)
      (Rendering|Components|Light|SetIntensity (Variables|Default|GetPortal_Light) 2.5e+04)
      (Variables|Default|SetisActivated true)
      (Variables|Default|SetinTransition false)
      (if (Variables|Default|GetlightningOn)
        (bind _returnvalue (Utilities|Time|SetTimerbyFunctionName 0 "F_Lightning" 1.0 true))
        (Variables|Default|SetTH_runningTimer _returnvalue)))))

(fn FDeactivateAltar
  (bind _sc_explosion_portal (Variables|Default|GetSC_Explosion_Portal))
  (if (> (Variables|Default|GettransitionTimer) 0.0)
    (Variables|Default|SettransitionTimer (- (Variables|Default|GettransitionTimer) 0.01))
    ;[1 1 1] Fade out Emission
    (Rendering|Material|SetScalarParameterValue (Variables|Default|GetMID_DemonicAltar) "Emission_Amount" (Variables|Default|GettransitionTimer) :!class /Script/Engine.MaterialInstanceDynamic)
    ;[1 1 1] Fade out portal light
    (Rendering|Components|Light|SetIntensity (Variables|Default|GetPortal_Light) (* (Variables|Default|GettransitionTimer) 2.5e+04))
    ;[1 1 1] Fade out Portal audio
    (Audio|Components|Audio|SetVolumeMultiplier _sc_explosion_portal (Variables|Default|GettransitionTimer) :!class /Script/Engine.AudioComponent)
    (else
      (Utilities|Time|ClearandInvalidateTimerbyHandle (Variables|Default|GetTH_runningTimer))
      (Audio|Components|Audio|Stop _sc_explosion_portal)
      (Audio|Components|Audio|SetVolumeMultiplier (Variables|Default|GetSC_Explosion_Portal) 1.0 :!class /Script/Engine.AudioComponent)
      (Variables|Default|SetisActivated false)
      (Variables|Default|SetinTransition false))))

(fn FLightning
  (if (<= (Variables|Default|GetlightningDelay) 0.0)
    (Variables|Default|SetlightningDelay (Math|Random|RandomFloatinRange 4.0 12.0))
    (Components|Activation|Activate (Variables|Default|GetPS_Lightning) false)
    (Components|Activation|Activate (Variables|Default|GetPS_Lightning_Runes) false)
    (Audio|Components|Audio|Play (Variables|Default|GetSC_Lightning) 0.0)
    (bind _returnvalue (Utilities|Time|SetTimerbyFunctionName 0 "F_LightFlicker" 0.04 true))
    (Variables|Default|SetTH_runningLightFlicker _returnvalue)
    (else
      (Variables|Default|SetlightningDelay (- (Variables|Default|GetlightningDelay) 1.0)))))

(fn FLightFlicker
  (if (<= (Variables|Default|GetflickerTimer) 4)
    (Rendering|Components|Light|SetIntensity (Variables|Default|GetLightning_Light) (* (Math|Random|RandomIntegerinRange 1 3) 5e+03))
    (Variables|Default|SetflickerTimer (+ (Variables|Default|GetflickerTimer) 1))
    (else
      (Rendering|Components|Light|SetIntensity (Variables|Default|GetLightning_Light) 0.0)
      (Variables|Default|SetflickerTimer 0)
      (Utilities|Time|ClearandInvalidateTimerbyHandle (Variables|Default|GetTH_runningLightFlicker)))))